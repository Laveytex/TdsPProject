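; Interactive-environment trap that spins continuously and grows its mesh into place shortly after play begins.
; BeginPlay flattens StaticMesh to zero X and Z scale, waits briefly, then calls Activate.
; Activate plays a timeline that drives the mesh's X and Z scale, preserving Y.
; Tick rotates the mesh and SMCylinder1 by a fixed step each frame, independent of delta time.
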(event Custom|Activate
  (bind (_direction _z _x) (Timeline|Timeline Play)
    (:Update
      (Transformation|SetWorldScale3D (Variables|Default|GetStaticMesh) (Math|Vector|MakeVector _z (.y (Variables|/Script/Engine.SceneComponent|GetRelativeScale3D (Variables|Default|GetStaticMesh))) _x)))))

(event EventBeginPlay
  (Transformation|SetWorldScale3D (Variables|Default|GetStaticMesh) (Math|Vector|MakeVector 0.0 (.y (Variables|/Script/Engine.SceneComponent|GetRelativeScale3D (Variables|Default|GetStaticMesh))) 0.0))
  (Utilities|FlowControl|Delay 1.0)
  (CallFunction|Activate))

(event EventTick
  (params (DeltaSeconds :type Float%20%28single-precision%29))
  (Transformation|AddWorldRotation (Variables|Default|GetSM_Cylinder1) "0.000000,3.000000,0.000000" false false))

(fn ConstructionScript)