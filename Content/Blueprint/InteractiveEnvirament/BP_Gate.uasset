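; BP_Gate is an automatic gate that opens when BP_Character enters its trigger box and closes when it leaves.
; Entry starts a one-second delay before a Timeline slides the Door along Z with audio cues, and exit reverses it.
; A gate that is not two-sided locks after that exit.
; Point light and dynamic-material lamp colors show state: yellow idle, green open, red locked.
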(event OnComponentBeginOverlap(Box)
  (params (OverlappedComponent :type Primitive%20Component%20Object%20Reference) (OtherActor :type Actor%20Object%20Reference) (OtherComp :type Primitive%20Component%20Object%20Reference) (OtherBodyIndex :type Integer) (bFromSweep :type Boolean) (SweepResult :type Hit%20Result%20Structure%20%28by%20ref%29))
  (Utilities|Casting|CastToBP_Character OtherActor)
  (if (not (Variables|Default|GetDoorLock))
    (Variables|Default|SetGateOpen true)
    (AddComponent|AddAudioComponent false)
    (Utilities|FlowControl|Delay 1.0)
    (CallFunction|DoorOpen)))

(event OnComponentEndOverlap(Box)
  (params (OverlappedComponent :type Primitive%20Component%20Object%20Reference) (OtherActor :type Actor%20Object%20Reference) (OtherComp :type Primitive%20Component%20Object%20Reference) (OtherBodyIndex :type Integer))
  (Utilities|Casting|CastToBP_Character OtherActor)
  (if (not (Variables|Default|GetDoorLock))
    (Variables|Default|SetGateOpen false)
    (CallFunction|DoorClose)
    (if (not (Variables|GateParametrs|GetIsTwoSide?))
      (Variables|Default|SetDoorLock true))))

(event Custom|DoorOpen
  (if (Variables|Default|GetGateOpen)
    (Components|Timeline|SetPlayRate (Variables|Default|GetTimeline) (Variables|GateParametrs|GetOpenSpeed))
    (AddComponent|AddAudioComponent false)
    (bind _newtrack_0 (Timeline|Timeline Play)
      (:Update
        (Transformation|SetRelativeLocation (Variables|Default|GetDoor) (Math|Vector|MakeVector 0.0 0.0 _newtrack_0) false false))
      (:Finished
        (if (Variables|Default|GetGateOpen)
          (CallFunction|SetLightColor "(R=0.173937,G=1.000000,B=0.000000,A=1.000000)")
          (CallFunction|DodyLightColor "(R=0.209845,G=1.000000,B=0.000000,A=1.000000)")
          (elif (Variables|Default|GetDoorLock)
            (CallFunction|SetLightColor "(R=1.000000,G=0.018845,B=0.000000,A=1.000000)")
            (CallFunction|DodyLightColor "(R=1.000000,G=0.000000,B=0.005189,A=1.000000)")
            (else
              (CallFunction|SetLightColor "(R=1.000000,G=0.956661,B=0.000000,A=1.000000)")
              (CallFunction|DodyLightColor "(R=1.000000,G=0.951255,B=0.000000,A=1.000000)"))))))
    (else
      (AddComponent|AddAudioComponent false)
      (Timeline|Timeline Reverse))))

(event Custom|DoorClose
  (if (Variables|Default|GetGateOpen)
    (Components|Timeline|SetPlayRate (Variables|Default|GetTimeline) (Variables|GateParametrs|GetOpenSpeed))
    (AddComponent|AddAudioComponent false)
    (bind _newtrack_0 (Timeline|Timeline Play)
      (:Update
        (Transformation|SetRelativeLocation (Variables|Default|GetDoor) (Math|Vector|MakeVector 0.0 0.0 _newtrack_0) false false))
      (:Finished
        (if (Variables|Default|GetGateOpen)
          (CallFunction|SetLightColor "(R=0.173937,G=1.000000,B=0.000000,A=1.000000)")
          (CallFunction|DodyLightColor "(R=0.209845,G=1.000000,B=0.000000,A=1.000000)")
          (elif (Variables|Default|GetDoorLock)
            (CallFunction|SetLightColor "(R=1.000000,G=0.018845,B=0.000000,A=1.000000)")
            (CallFunction|DodyLightColor "(R=1.000000,G=0.000000,B=0.005189,A=1.000000)")
            (else
              (CallFunction|SetLightColor "(R=1.000000,G=0.956661,B=0.000000,A=1.000000)")
              (CallFunction|DodyLightColor "(R=1.000000,G=0.951255,B=0.000000,A=1.000000)"))))))
    (else
      (AddComponent|AddAudioComponent false)
      (Timeline|Timeline Reverse))))

(event EventBeginPlay
  (CallFunction|SetLightColor "(R=1.000000,G=0.906927,B=0.000000,A=1.000000)")
  (Rendering|Components|Light|SetIntensity (Variables|Default|GetPointLight) (Variables|GateParametrs|GetLightIntensity))
  (CallFunction|DodyLightColor "(R=1.000000,G=0.887260,B=0.000000,A=1.000000)"))

(fn ConstructionScript)

(fn SetLightColor
  (params (NewLightColor :type Linear%20Color%20Structure))
  (Rendering|Components|Light|SetLightColor (Variables|Default|GetPointLight) NewLightColor true))

(fn DodyLightColor
  (params (Value :type Linear%20Color%20Structure))
  (bind _returnvalue (Rendering|Material|CreateDynamicMaterialInstance (Variables|Default|GetFlashLight) 0 "/Game/Enviroment/Materials/M_LightInstanse.M_LightInstanse" "Color" :!class /Script/Engine.PrimitiveComponent))
  (Rendering|Material|SetVectorParameterValue _returnvalue "Color" Value :!class /Script/Engine.MaterialInstanceDynamic))