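; Top-down player character Blueprint handling movement modes, stamina-limited sprint, camera control and weapon animations.
; Input sets flags for ChangeMovementState; sprint requires forward movement, with looping timers draining and refilling stamina.
; Mouse wheel zooms the boom directly or in timed steps, while Tick pans it toward the cursor when aiming, scaled by zoom, or eases it back.
; Reload events play rate-adjusted montages; hard-wired keys trigger fire montages and camera shake.
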(event EventWeaponReloadEndBP
  (Variables|Default|SetbIsReload? false))

(event EventWeaponReloadStartBP
  (params (Anim :type Anim%20Montage%20Object%20Reference))
  (bind _returnvalue (Class|TDSCharacter|GetCurrentWeapon))
  (bind _output_get (Variables|Default|SetReloadAnim Anim))
  (if (not (Variables|Default|GetbIsReload?))
    (Variables|Default|SetIn%20Play%20Rate (/ (Variables|/Script/TDS.WeaponDefault|GetReloadTime _returnvalue) (Animation|GetPlayLength _output_get)))
    (Animation|PlayAnimMontage Anim (Variables|Default|GetIn%20Play%20Rate) "None")
    (Variables|Default|SetbIsReload? true)))

(event EventTick
  (params (DeltaSeconds :type Float%20%28single-precision%29))
  (CallFunction|CameraMoveZoom DeltaSeconds))

(event Input|ActionEvents|InputActionMovementModChangeSprint
  (params (Key :type Key%20Structure :default "None"))
  (:Pressed
    (CallFunction|Sprint)
    (Class|TDSCharacter|ChangeMovementState :!label _label)
    (Development|PrintString (Utilities|String|EnumtoString (Variables|Default|GetMovementState))))
  (:Released
    (CallFunction|SprintReleased)
    (goto _label)))

(event Input|ActionEvents|InputActionMovementModChangeWalk
  (params (Key :type Key%20Structure :default "None"))
  (:Pressed
    (Variables|Default|SetWalkEnabled true)
    (Class|TDSCharacter|ChangeMovementState :!label _label)
    (Development|PrintString (Utilities|String|EnumtoString (Variables|Default|GetMovementState))))
  (:Released
    (Variables|Default|SetWalkEnabled false)
    (goto _label)))

(event Input|ActionEvents|InputActionMovementModChangeCrouch
  (params (Key :type Key%20Structure :default "None"))
  (:Pressed
    (Variables|Default|SetCroucnEnabled true)
    (Class|TDSCharacter|ChangeMovementState :!label _label)
    (Development|PrintString (Utilities|String|EnumtoString (Variables|Default|GetMovementState))))
  (:Released
    (Variables|Default|SetCroucnEnabled false)
    (goto _label)))

(event Input|AxisEvents|InputAxisMouseWheel
  (params (AxisValue :type Float%20%28single-precision%29))
  (if (Variables|Camera|GetSlideWithSmooth)
    (CallFunction|CameraSideSmooth AxisValue)
    (else
      (CallFunction|CameraSideLegasy AxisValue))))

(event Input|KeyboardEvents|F
  (params (Key :type Key%20Structure :default "None"))
  (:Pressed
    (CallFunction|CameraShakeIvent)))

(event Input|MouseEvents|RightMouseButton
  (params (Key :type Key%20Structure :default "None"))
  (:Pressed
    (Variables|Default|SetAimEnabled true)
    (Class|TDSCharacter|ChangeMovementState :!label _label)
    (Development|PrintString (Utilities|String|EnumtoString (Variables|Default|GetMovementState))))
  (:Released
    (Variables|Default|SetAimEnabled false)
    (goto _label)))

(event Input|KeyboardEvents|SpaceBar
  (params (Key :type Key%20Structure :default "None"))
  (bind _mesh (Variables|Character|GetMesh))
  (:Pressed
    (if (Variables|Default|GetAimEnabled)
      (Animation|Montage|PlayMontage _mesh "/Game/Blueprint/Character/Mannequins/Animations/Quinn/Aim/Fire_Rifle_Ironsights_Montage.Fire_Rifle_Ironsights_Montage")
      (else
        (Animation|Montage|PlayMontage _mesh "/Game/Blueprint/Character/Mannequins/Animations/Quinn/Aim/Fire_Rifle_Hip_Montage.Fire_Rifle_Hip_Montage")))))

(fn ConstructionScript
  (bind _cameraboom (Variables|Default|GetCameraBoom))
  (Variables|/Script/Engine.SpringArmComponent|SetTargetArmLength _cameraboom (Variables|CameraParametrs|GetCameraHeight))
  (Transformation|SetRelativeRotation _cameraboom (Variables|CameraParametrs|GetRotatorCamera) false false)
  (Variables|/Script/Engine.SpringArmComponent|SetbEnableCameraLag _cameraboom (Variables|CameraParametrs|GetFlow))
  (Variables|/Script/Engine.SpringArmComponent|SetCameraLagSpeed _cameraboom (Variables|CameraParametrs|GetCoefSmooth)))

(fn CameraShakeIvent
  (Camera|PlayWorldCameraShake "/Game/Blueprint/Game/BP_CameraShake.BP_CameraShake_C" (Transformation|GetWorldLocation (Variables|Default|GetTopDownCameraComponent)) 0.0 3e+01))

(fn CameraSideLegasy
  (params (InputPin :type Float%20%28double-precision%29))
  (bind _cameraboom (Variables|Default|GetCameraBoom))
  (if (Variables|Camera|GetSlideDone)
    (if (!= InputPin 0.0)
      (Variables|/Script/Engine.SpringArmComponent|SetTargetArmLength _cameraboom (Math|Float|Clamp(Float) (+ (Variables|/Script/Engine.SpringArmComponent|GetTargetArmLength _cameraboom) (* (* InputPin -1.0) (Variables|Camera|GetCameraHeightChangeDistance))) (Variables|Camera|GetHeightCameraMin) (Variables|Camera|GetHeightCameraMax))))))

(fn CameraSideSmothTick
  (bind _heightcameraheightchangeslidestapdistance (Variables|Camera|GetHeightCameraHeightChangeSlideStapDistance))
  (bind _cameraboom (Variables|Default|GetCameraBoom))
  (bind _output_get (Variables|Camera|SetCurrentSlideDistance (+ (Variables|Camera|GetCurrentSlideDistance) _heightcameraheightchangeslidestapdistance)))
  (Variables|/Script/Engine.SpringArmComponent|SetTargetArmLength _cameraboom (Math|Float|Clamp(Float) (Math|Float|SelectFloat (- (Variables|/Script/Engine.SpringArmComponent|GetTargetArmLength _cameraboom) _heightcameraheightchangeslidestapdistance) (+ (Variables|/Script/Engine.SpringArmComponent|GetTargetArmLength _cameraboom) _heightcameraheightchangeslidestapdistance) (Variables|Camera|GetSlideUp)) (Variables|Camera|GetHeightCameraMin) (Variables|Camera|GetHeightCameraMax)))
  (if (>= _output_get (Variables|Camera|GetCameraHeightChangeDistance))
    (Variables|Camera|SetCurrentSlideDistance 0.0)
    (Variables|Camera|SetSlideDone true)
    (Utilities|Time|ClearandInvalidateTimerbyHandle (Variables|Camera|GetSlideTimer))))

(fn CameraSideSmooth
  (params (InputPin :type Float%20%28double-precision%29))
  (if (Variables|Camera|GetSlideDone)
    (if (!= InputPin 0.0)
      (if (> InputPin 0.0)
        (Variables|Camera|SetSlideUp true)
        (else
          (Variables|Camera|SetSlideUp false)))
      (Variables|Camera|SetSlideDone false)
      (bind _returnvalue (Utilities|Time|SetTimerbyFunctionName 0 "CameraSideSmothTick" (Variables|Camera|GetTimer%20Step) true))
      (Variables|Camera|SetSlideTimer _returnvalue))))

(fn Sprint
  (if (Utilities|Operators|EqualEqual (Math|Vector|Normalize (Transformation|GetActorForwardVector)) (Math|Vector|Normalize (Variables|/Script/Engine.MovementComponent|GetVelocity (Variables|Character|GetCharacterMovement))) 0.2)
    (if (> (Variables|Stamina|GetStamina) 0.0)
      (Variables|Default|SetSprintRunEnabled true)
      (Class|TDSCharacter|ChangeMovementState)
      (bind _returnvalue (Utilities|Time|SetTimerbyFunctionName 0 "StaminaSpend" 0.01 true))
      (Variables|Stamina|SetStaminaTimer _returnvalue))))

(fn StaminaSpend
  (if (Variables|Default|GetSprintRunEnabled)
    (if (> (Variables|Stamina|GetStamina) 0.0)
      (Variables|Stamina|SetStamina (- (Variables|Stamina|GetStamina) (Variables|Stamina|GetStaminaSpendStap)))
      (else
        (Variables|Default|SetSprintRunEnabled false)
        (Class|TDSCharacter|ChangeMovementState)
        (CallFunction|SprintReleased)))))

(fn StaminaRecycle
  (if (not (Variables|Default|GetSprintRunEnabled))
    (Class|TDSCharacter|ChangeMovementState)
    (if (< (Variables|Stamina|GetStamina) (Variables|Stamina|GetStaminaMax))
      (Variables|Stamina|SetStamina (+ (Variables|Stamina|GetStamina) (Variables|Stamina|GetStaminaSpendStap))))))

(fn SprintReleased
  (Variables|Default|SetSprintRunEnabled false)
  (bind _returnvalue (Utilities|Time|SetTimerbyFunctionName 0 "StaminaRecycle" 0.01 true))
  (Variables|Stamina|SetStaminaTimer _returnvalue))

(fn CameraMoveZoom
  (params (DeltaTime :type Float%20%28single-precision%29))
  (bind _capsulecomponent (Variables|Default|GetCapsuleComponent))
  (bind _cameraboom (Variables|Default|GetCameraBoom))
  (bind _cameraboom_2 (Variables|Default|GetCameraBoom))
  (bind _returnvalue (Transformation|GetWorldLocation _capsulecomponent))
  (bind _returnvalue_2 (Transformation|GetWorldLocation _cameraboom))
  (bind _returnvalue_3 (Class|TDSCharacter|GetCursortoWorld))
  (Variables|CameraZoomMoveParametrs|SetCameraClampedHeight (Math|Float|MapRangeClamped (Variables|/Script/Engine.SpringArmComponent|GetTargetArmLength (Variables|Default|GetCameraBoom)) (Variables|Camera|GetHeightCameraMin) (Variables|Camera|GetHeightCameraMax) 0.5 1.0))
  (Variables|CameraZoomMoveParametrs|SetDistanceCameraBoomChar (Math|Vector|VectorLengthXY (- _returnvalue (Transformation|GetWorldLocation _returnvalue_3))))
  (if (or (Utilities|Enum|Equal(Enum) (Variables|Default|GetMovementState) "AimWalk_State") (Utilities|Enum|Equal(Enum) (Variables|Default|GetMovementState) "AimRun_State"))
    (if (> (Variables|CameraZoomMoveParametrs|GetDistanceCameraBoomChar) (* (Variables|CameraZoomMoveParametrs|GetCameraClampedHeight) (Variables|CameraZoomMoveParametrs|GetfMinClampDistanceLogicMouseCursorStart)))
      (if (not (> (Math|Vector2D|Vector2DLength (Math|Conversions|ToVector2D(Vector) (- (Transformation|GetWorldLocation (Variables|Default|GetCameraBoom)) _returnvalue))) (* (Variables|CameraZoomMoveParametrs|GetCameraClampedHeight) (Variables|CameraZoomMoveParametrs|GetfMaxClampDistanceLogicMouseCursorStart))))
        (Transformation|SetWorldLocation _cameraboom (Math|Vector|MakeVector (+ (.x _returnvalue_2) (.X (Math|Vector2D|BreakVector2D (* (Math|Vector2D|Normalize2D (Math|Conversions|ToVector2D(Vector) (Math|Vector|GetForwardVector (Math|Rotator|FindLookatRotation _returnvalue (Transformation|GetWorldLocation _returnvalue_3))))) "(X=6.000000,Y=6.000000)")))) (+ (.y _returnvalue_2) (.Y (Math|Vector2D|BreakVector2D (* (Math|Vector2D|Normalize2D (Math|Conversions|ToVector2D(Vector) (Math|Vector|GetForwardVector (Math|Rotator|FindLookatRotation _returnvalue (Transformation|GetWorldLocation _returnvalue_3))))) "(X=6.000000,Y=6.000000)")))) (.z _returnvalue_2)) false false))
      (else
        (Transformation|SetWorldLocation _cameraboom_2 (Math|Interpolation|VInterpTo (Transformation|GetWorldLocation _cameraboom_2) (Transformation|GetWorldLocation (Variables|Default|GetCapsuleComponent)) DeltaTime (Variables|CameraZoomMoveParametrs|GetFSpeedChangeLocationCameraToDefault)) false false :!label _label)))
    (else
      (goto _label))))